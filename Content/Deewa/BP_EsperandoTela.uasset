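; BP_EsperandoTela is an overlap volume that ends the game once enough actors are inside it at the same time.
; It raises the Salida counter on each begin overlap and lowers it on each end overlap, without filtering by actor type.
; When the count rises above four, it casts the game mode to BP_GM_Gameplay and calls FinishGame.
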(event Collision|EventActorBeginOverlap
  (params (OtherActor :type Actor%20Object%20Reference))
  (Math|Integer|IncrementInt (Variables|Default|GetSalida)
    (:%20%20
      (if (> (Variables|Default|GetSalida) 4)
        (bind _asbp_gm_gameplay (Utilities|Casting|CastToBP_GM_Gameplay (Game|GetGameMode)))
        (Default|FinishGame _asbp_gm_gameplay)))))

(event Collision|EventActorEndOverlap
  (params (OtherActor :type Actor%20Object%20Reference))
  (Math|Integer|DecrementInt (Variables|Default|GetSalida)))

(fn ConstructionScript)
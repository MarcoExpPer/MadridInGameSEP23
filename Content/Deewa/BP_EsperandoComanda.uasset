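; BP_EsperandoComanda ("waiting for order") is an overlap zone that ends the game when it gets too crowded.
; An Entrada counter rises on each actor begin overlap and falls on each end overlap, with no filtering by actor type.
; Once the count exceeds three, it casts the game mode to BP_GM_Gameplay and calls FinishGame.
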(event Collision|EventActorBeginOverlap
  (params (OtherActor :type Actor%20Object%20Reference))
  (Math|Integer|IncrementInt (Variables|Default|Getentrada)
    (:%20%20
      (if (> (Variables|Default|Getentrada) 3)
        (bind _asbp_gm_gameplay (Utilities|Casting|CastToBP_GM_Gameplay (Game|GetGameMode)))
        (Default|FinishGame _asbp_gm_gameplay)))))

(event Collision|EventActorEndOverlap
  (params (OtherActor :type Actor%20Object%20Reference))
  (Math|Integer|DecrementInt (Variables|Default|Getentrada)))

(fn ConstructionScript)
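; Customer character that walks into a waiting line and requests a randomly generated order.
; GoToWaitLine picks a pattern, left/right side and tint from the level's material generators and tint machines, shows them on the help widget and registers with the gameplay GameMode's queue.
; Tick moves it along Y, with paired DoOnce nodes switching walk/idle animation and rotation.
; Tagged overlaps count checkpoints or halt it; key 2 resumes customers past their first checkpoint.
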(event Custom|GoToWaitLine
  (bind _resultpattern_ (Variables|Default|GetresultPattern?))
  (Variables|Default|SetMove true)
  (CallFunction|ObtainPatron)
  (Components|DestroyComponent (Variables|Default|GetWidgetEmissive))
  (Default|UpdateIcon (Variables|Default|GetWG_customerHelp) (select (Variables|Default|GetresultIsLeft?) (.spriteleft _resultpattern_) (.spriteright _resultpattern_)))
  (Default|UpdateColor (Variables|Default|GetWG_customerHelp) (Variables|Default|GetresultTint?))
  (Variables|/Script/UMG.Widget|SetRenderOpacity (Variables|Default|GetWG_customerHelp) 1.0)
  (Default|AddCustomertoQueue (Variables|Default|GetBP_GM_Gameplay) self))

(event Collision|EventActorBeginOverlap
  (params (OtherActor :type Actor%20Object%20Reference))
  (bind _returnvalue (Actor|ActorHasTag OtherActor "Tela"))
  (bind _box (Variables|Default|GetBox))
  (if _returnvalue
    (Math|Integer|IncrementInt (Variables|Default|GetCheckpointCount)
      (:%20%20
        _)))
  (if (not (or (Actor|ActorHasTag OtherActor "Comanda") _returnvalue))
    (Transformation|SetWorldScale3D _box (* (Transformation|GetWorldScale _box) 0.97))
    (if (Actor|ActorHasTag OtherActor "Checkpoint")
      (Utilities|FlowControl|Delay 0.2)
      (Math|Integer|IncrementInt (Variables|Default|GetCheckpointCount)
        (:%20%20
          (Variables|Default|SetMove false)))
      (else
        (Variables|Default|SetMove false)))))

(event EventTick
  (params (DeltaSeconds :type Float%20%28single-precision%29))
  (if (Variables|Default|GetMove)
    (Transformation|AddActorWorldOffset (Math|Vector|MakeVector 0.0 (* DeltaSeconds (Variables|Default|GetClientSpeed)) 0.0))
    (Utilities|FlowControl|DoOnce false :!label _label
      (:Completed
        (Components|Animation|PlayAnimation (Variables|Default|GetSkeletalMesh) "/Game/Deewa/animation/ClienteWalk_Anim.ClienteWalk_Anim" true)
        (Transformation|AddWorldRotation (Variables|Default|GetSkeletalMesh) "0.000000,-90.000000,0.000000" false false)
        (goto _label_2 Reset)))
    (else
      (Utilities|FlowControl|DoOnce false :!label _label_2
        (:Completed
          (Components|Animation|PlayAnimation (Variables|Default|GetSkeletalMesh) "/Game/Deewa/animation/ClienteIdle_Anim.ClienteIdle_Anim" true)
          (Transformation|AddWorldRotation (Variables|Default|GetSkeletalMesh) "0.000000,90.000000,0.000000" false false)
          (goto _label Reset))))))

(event EventBeginPlay
  (Input|EnableInput (Game|GetPlayerController 0))
  (bind _aswg_customer_help (Utilities|Casting|CastToWG_customerHelp (UserInterface|GetWidget (Variables|Default|GetWidget))))
  (bind _output_get (Variables|Default|SetWG_customerHelp _aswg_customer_help))
  (Variables|/Script/UMG.Widget|SetRenderOpacity _output_get 0.0)
  (bind _asbp_gm_gameplay (Utilities|Casting|CastToBP_GM_Gameplay (Game|GetGameMode)))
  (Variables|Default|SetBP_GM_Gameplay _asbp_gm_gameplay))

(event Collision|EventActorEndOverlap
  (params (OtherActor :type Actor%20Object%20Reference)))

(event Input|KeyboardEvents|2
  (params (Key :type Key%20Structure))
  (:Pressed
    (bind _outactors (Actor|GetAllActorsOfClass "BP_ClientesPj_C"))
    (for _array_element _outactors
      (if (> (Variables|BP_ClientesPj_C|GetCheckpointCount _array_element) 1)
        (Variables|BP_ClientesPj_C|SetMove _array_element true)))))

(fn ConstructionScript)

(fn ObtainPatron
  (bind _availablecolors (LocalVariables|GetavailableColors))
  (bind _outactors (Actor|GetAllActorsOfClass "/Game/Marco/Interactuables/BP_BaseMaterialGenerator.BP_BaseMaterialGenerator_C"))
  (for _array_element _outactors
    (Utilities|Array|AddUnique (LocalVariables|GetavailableRaws) (Variables|/Game/Marco/Interactuables/BP_BaseMaterialGenerator.BP_BaseMaterialGenerator_C|GetRawMatData _array_element)))
  (Variables|Default|SetresultPattern? (Utilities|Array|Get(acopy) (LocalVariables|GetavailableRaws) (Math|Random|RandomIntegerinRange 0 (- (Utilities|Array|Length (LocalVariables|GetavailableRaws)) 1))))
  (Variables|Default|SetresultIsLeft? (Math|Random|RandomBool))
  (bind _outactors_2 (Actor|GetAllActorsOfClass "/Game/Marco/Interactuables/BP_TintMachine.BP_TintMachine_C"))
  (for _array_element_2 _outactors_2
    (Utilities|Array|AddUnique _availablecolors (Variables|/Game/Marco/Interactuables/BP_TintMachine.BP_TintMachine_C|GetleftTint _array_element_2))
    (Utilities|Array|AddUnique _availablecolors (Variables|/Game/Marco/Interactuables/BP_TintMachine.BP_TintMachine_C|GetrightTint _array_element_2)))
  (Variables|Default|SetresultTint? (Utilities|Array|Get(acopy) (LocalVariables|GetavailableColors) (Math|Random|RandomIntegerinRange 0 (- (Utilities|Array|Length (LocalVariables|GetavailableColors)) 1))))
  (return))
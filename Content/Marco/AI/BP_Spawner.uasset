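; BP_Spawner spawns customers and manages their two queues, waiting and end, until they leave.
; A looping timer spawns customers, substituting named characters or toppling random mannequins at set counts, and updates crowd-murmur volume by headcount.
; AI MoveTo walks customers along waypoint arrays, shifting each line forward as its front leaves.
; An overfull queue ends the game; StartGame spawns a boss, and tutorial exits require a happy customer.
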(event Custom|SpawnNormalActor
  (bind _returnvalue (Transformation|GetActorTransform))
  (Math|Integer|IncrementInt (Variables|Default|GettotalEnemyCount)
    (:%20%20
      (bind _result (Math|Integer|IncrementInt (Variables|Default|GetenemyCount))
        (:%20%20
          (CallFunction|UpdateCrowdSound _result)
          (Variables|Default|SetclassToSpawn "/Game/Marco/AI/BP_MyCustomer.BP_MyCustomer_C")
          (Audio|PlaySound2D "/Game/Audio/Raw/doorbell.doorbell" 1.0 1.0 0.0 0 0)
          (switch int (Variables|Default|GettotalEnemyCount)
            (:Default
              _)
            (:0
              _)
            (:1
              _)
            (:2
              _)
            (:3
              (Variables|Default|SetclassToSpawn "/Game/Marco/AI/BP_Carlos_Lujofeld.BP_Carlos_Lujofeld_C"))
            (:4
              (CallFunction|ActivateMannequin))
            (:5
              _)
            (:6
              (Variables|Default|SetclassToSpawn "/Game/Marco/AI/BP_Cristiana_Pedruscos.BP_Cristiana_Pedruscos_C"))
            (:7
              (CallFunction|ActivateMannequin))
            (:8
              _)
            (:9
              (CallFunction|ActivateMannequin))
            (:10
              _))
          (if (>= (Utilities|Array|Length (Variables|Default|GetcustomersWaiting)) 3)
            (bind _asbp_gm_gameplay (Utilities|Casting|CastToBP_GM_Gameplay (Game|GetGameMode)))
            (Default|FinishGame _asbp_gm_gameplay)
            (else
              (bind _returnvalue_2 (Game|SpawnActorfromClass (Variables|Default|GetclassToSpawn) (Math|Transform|MakeTransform (.location _returnvalue) (.rotation _returnvalue) "1.500000,1.500000,1.500000") "AlwaysSpawn" 0 true 0))
              (Variables|/Game/Marco/AI/BP_MyCustomer.BP_MyCustomer_C|SetBP_spawner _returnvalue_2 self)
              (bind _returnvalue_3 (Utilities|Array|Add (Variables|Default|GetcustomersWaiting) _returnvalue_2))
              (bind _output_get (Variables|/Game/Marco/AI/BP_MyCustomer.BP_MyCustomer_C|SettargetIndex _returnvalue_2 _returnvalue_3))
              (if (== _output_get 0)
                (Default|ShowExclamation _returnvalue_2))
              (AI|AIMoveTo (AI|GetAIController _returnvalue_2) "0, 0, 0" (Utilities|Array|Get(acopy) (Variables|Default|GetwaitingWaypoints) _output_get) 5.0 "Disable" "Default" true true))))))))

(event Custom|CustomEvent
  (CallFunction|SpawnNormalActor))

(event Custom|StartSpawningClients
  (params (timeToSpawn :type Float%20%28double-precision%29) (spawnOnCall :type Boolean))
  (if spawnOnCall
    (CallFunction|SpawnNormalActor))
  (Utilities|Time|ClearandInvalidateTimerbyHandle (Variables|Default|GetclientTimer))
  (bind _returnvalue (Utilities|Time|SetTimerbyEvent (delegate Custom|CustomEvent) timeToSpawn true))
  (Variables|Default|SetclientTimer _returnvalue))

(event Custom|AdvanceOneFromWaiting
  (bind _customerswaiting (Variables|Default|GetcustomersWaiting))
  (bind _output (Utilities|Array|Get(acopy) _customerswaiting))
  (if (>= (Utilities|Array|Length (Variables|Default|GetcustomersAtTheEnd)) 5)
    (bind _asbp_gm_gameplay (Utilities|Casting|CastToBP_GM_Gameplay (Game|GetGameMode)))
    (Default|FinishGame _asbp_gm_gameplay)
    (else
      (Default|ShowProduct _output)
      (Components|Movement|StopMovementImmediately (Variables|/Script/Engine.Character|GetCharacterMovement _output))
      (bind _returnvalue (Utilities|Array|Add (Variables|Default|GetcustomersAtTheEnd) _output))
      (bind _output_get (Variables|/Game/Marco/AI/BP_MyCustomer.BP_MyCustomer_C|SettargetIndex _output _returnvalue))
      (AI|AIMoveTo (AI|GetAIController _output) "0, 0, 0" (Utilities|Array|Get(acopy) (Variables|Default|GettheEndWaypoints) _output_get) 5.0 "Disable" "Default" true true
        (:then
          (Utilities|Array|RemoveIndex (Variables|Default|GetcustomersWaiting))
          (for _array_element (Variables|Default|GetcustomersWaiting)
            (bind _result (Math|Integer|DecrementInt (Variables|/Game/Marco/AI/BP_MyCustomer.BP_MyCustomer_C|GettargetIndex _array_element))
              (:%20%20
                (Components|Movement|StopMovementImmediately (Variables|/Script/Engine.Character|GetCharacterMovement _array_element))
                (if (== _result 0)
                  (Default|ShowExclamation _array_element))
                (AI|AIMoveTo (AI|GetAIController _array_element) "0, 0, 0" (Utilities|Array|Get(acopy) (Variables|Default|GetwaitingWaypoints) _result) 5.0 "Disable" "Default" true true)))))))))

(event Custom|SendCustomerOutside
  (params (happy :type Boolean))
  (bind _customersattheend (Variables|Default|GetcustomersAtTheEnd))
  (bind _output (Utilities|Array|Get(acopy) _customersattheend))
  (if (Variables|Default|GetinTutorial)
    (if happy
      (Variables|Default|SetinTutorial false)
      (Utilities|IsValid (Variables|Default|GetlastCustomer) :!label _label
        (:Is%20Valid
          (Actor|DestroyActor (Variables|Default|GetlastCustomer)))
        (:Is%20Not%20Valid
          _))
      (bind _output_get (Variables|Default|SetlastCustomer _output))
      (Components|Movement|StopMovementImmediately (Variables|/Script/Engine.Character|GetCharacterMovement _output_get))
      (AI|AIMoveTo (AI|GetAIController _output) "0, 0, 0" (Variables|Default|GetdespawnCheckpoint) 2.0 "Disable" "Default" true true
        (:then
          (Utilities|Array|RemoveIndex (Variables|Default|GetcustomersAtTheEnd))
          (for _array_element (Variables|Default|GetcustomersAtTheEnd)
            (bind _result (Math|Integer|DecrementInt (Variables|/Game/Marco/AI/BP_MyCustomer.BP_MyCustomer_C|GettargetIndex _array_element))
              (:%20%20
                (Components|Movement|StopMovementImmediately (Variables|/Script/Engine.Character|GetCharacterMovement _array_element))
                (AI|AIMoveTo (AI|GetAIController _array_element) "0, 0, 0" (Utilities|Array|Get(acopy) (Variables|Default|GettheEndWaypoints) _result) 5.0 "Disable" "Default" true true)))))))
    (else
      (bind _result_2 (Math|Integer|DecrementInt (Variables|Default|GetenemyCount))
        (:%20%20
          (CallFunction|UpdateCrowdSound _result_2)
          (goto _label))))))

(event Custom|StartGame
  (bind _returnvalue (Transformation|GetActorTransform))
  (bind _returnvalue_2 (Game|SpawnActorfromClass "/Game/Marco/AI/BP_Boss.BP_Boss_C" (Math|Transform|MakeTransform (.location _returnvalue) (.rotation _returnvalue) "1.000000,1.000000,1.000000") "Undefined" 0 false 0))
  (bind _returnvalue_3 (Utilities|Array|Add (Variables|Default|GetcustomersWaiting) _returnvalue_2))
  (bind _output_get (Variables|/Game/Marco/AI/BP_MyCustomer.BP_MyCustomer_C|SettargetIndex _returnvalue_2 _returnvalue_3))
  (AI|AIMoveTo (AI|GetAIController _returnvalue_2) "0, 0, 0" (Utilities|Array|Get(acopy) (Variables|Default|GetwaitingWaypoints) _output_get) 5.0 "Disable" "Default" true true
    (:then
      (Audio|PlaySound2D "/Game/Audio/Raw/doorbell.doorbell" 1.0 1.0 0.0 0 0))))

(event EventBeginPlay
  (bind _returnvalue (Transformation|GetActorTransform))
  (if (Variables|Default|GetautomaticStart)
    (bind _returnvalue_2 (Game|SpawnActorfromClass "/Game/Marco/AI/BP_Boss.BP_Boss_C" (Math|Transform|MakeTransform (.location _returnvalue) (.rotation _returnvalue) "1.000000,1.000000,1.000000") "Undefined" 0 false 0))
    (bind _returnvalue_3 (Utilities|Array|Add (Variables|Default|GetcustomersWaiting) _returnvalue_2))
    (bind _output_get (Variables|/Game/Marco/AI/BP_MyCustomer.BP_MyCustomer_C|SettargetIndex _returnvalue_2 _returnvalue_3))
    (AI|AIMoveTo (AI|GetAIController _returnvalue_2) "0, 0, 0" (Utilities|Array|Get(acopy) (Variables|Default|GetwaitingWaypoints) _output_get) 5.0 "Disable" "Default" true true
      (:then
        (Audio|PlaySound2D "/Game/Audio/Raw/doorbell.doorbell" 1.0 1.0 0.0 0 0)))))

(fn ConstructionScript)

(fn ActivateMannequin
  (bind _outactors (Actor|GetAllActorsOfClass "/Game/Marco/BP_Manequin.BP_Manequin_C"))
  (for _array_element _outactors
    (if (Variables|/Game/Marco/BP_Manequin.BP_Manequin_C|GetcanBeActivated _array_element)
      (Utilities|Array|Add (LocalVariables|GetavailableManq) _array_element)))
  (if (!= (Utilities|Array|Length (LocalVariables|GetavailableManq)) 0)
    (Default|StartFalling (Utilities|Array|Get(acopy) (LocalVariables|GetavailableManq) (Math|Random|RandomIntegerinRange 0 (- (Utilities|Array|Length (LocalVariables|GetavailableManq)) 1))))
    (return)
    (else
      (return))))

(fn UpdateCrowdSound
  (params (nCustomers :type Integer))
  (Utilities|IsValid (Variables|Default|GetcrowdSound)
    (:Is%20Valid
      (Audio|Components|Audio|SetVolumeMultiplier (Variables|Default|GetcrowdSound) (Utilities|GetSoundVolume nCustomers) :!class /Script/Engine.AudioComponent))
    (:Is%20Not%20Valid
      (bind _returnvalue (Audio|SpawnSound2D "/Game/Audio/Raw/Ambiente_murmullo.Ambiente_murmullo" (Utilities|GetSoundVolume nCustomers) 1.0 0.0 0 false false))
      (Variables|Default|SetcrowdSound _returnvalue))))
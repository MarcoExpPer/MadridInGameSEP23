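; BP_Boss is a boss AI actor that reports its encounter through game mode dialogue and signals when it finishes.
; It sets a dialogue line shortly after BeginPlay, on getting a command, and on exiting, with the exit line depending on IsHappy.
; A happy exit also shows a happy emotion widget on WidgetPattern and calls BossFinished on BP_GM_Gameplay, while an unhappy exit only changes the dialogue.
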(event EventBeginPlay
  (|CallParentFunction)
  (Utilities|FlowControl|Delay 0.2)
  (bind _asbp_gm_gameplay (Utilities|Casting|CastToBP_GM_Gameplay (Game|GetGameMode)))
  (Default|SetDialog (Variables|/Game/Marco/BP_GM_Gameplay.BP_GM_Gameplay_C|GetDialogue _asbp_gm_gameplay) "NewEnumerator6"))

(event Collision|EventActorBeginOverlap
  (params (OtherActor :type Actor%20Object%20Reference))
  (|CallParentFunction OtherActor) ; This node is disabled and will not be called.\nDrag off pins to build functionality.
)

(event EventTick
  (params (DeltaSeconds :type Float%20%28single-precision%29))
  (|CallParentFunction DeltaSeconds) ; This node is disabled and will not be called.\nDrag off pins to build functionality.
)

(event EventOnExiting
  (params (isHappy :type Boolean) (is%20puta :type Boolean))
  (if isHappy
    (bind _returnvalue (UserInterface|CreateWidget "/Game/Marco/HUD/emotions/WG_EmotionsShow.WG_EmotionsShow_C"))
    (UserInterface|SetWidget (Variables|Default|GetWidgetPattern) _returnvalue)
    (Default|ActivateHappy _returnvalue)
    (bind _asbp_gm_gameplay (Utilities|Casting|CastToBP_GM_Gameplay (Game|GetGameMode)))
    (Default|SetDialog (Variables|/Game/Marco/BP_GM_Gameplay.BP_GM_Gameplay_C|GetDialogue _asbp_gm_gameplay) "NewEnumerator9")
    (Default|BossFinished _asbp_gm_gameplay)
    (else
      (bind _asbp_gm_gameplay_2 (Utilities|Casting|CastToBP_GM_Gameplay (Game|GetGameMode)))
      (Default|SetDialog (Variables|/Game/Marco/BP_GM_Gameplay.BP_GM_Gameplay_C|GetDialogue _asbp_gm_gameplay_2) "NewEnumerator8"))))

(event EventOnGettingCommand
  (bind _asbp_gm_gameplay (Utilities|Casting|CastToBP_GM_Gameplay (Game|GetGameMode)))
  (Default|SetDialog (Variables|/Game/Marco/BP_GM_Gameplay.BP_GM_Gameplay_C|GetDialogue _asbp_gm_gameplay) "NewEnumerator7"))

(fn ConstructionScript
  (|CallParentFunction))
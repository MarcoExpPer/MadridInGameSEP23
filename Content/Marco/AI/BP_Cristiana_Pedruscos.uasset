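; BP_Cristiana_Pedruscos is a character-specific Blueprint, filed under AI, that triggers dialogue for Cristiana Pedruscos.
; Its command and exit events each cast the game mode to BP_GM_Gameplay and set a different enum-selected line on its Dialogue.
; The exit line plays only when the event's boolean flag is false.
; BeginPlay, overlap, Tick and construction add no logic of their own.
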(event EventBeginPlay
  (|CallParentFunction) ; This node is disabled and will not be called.\nDrag off pins to build functionality.
)

(event Collision|EventActorBeginOverlap
  (params (OtherActor :type Actor%20Object%20Reference))
  (|CallParentFunction OtherActor) ; This node is disabled and will not be called.\nDrag off pins to build functionality.
)

(event EventTick
  (params (DeltaSeconds :type Float%20%28single-precision%29))
  (|CallParentFunction DeltaSeconds) ; This node is disabled and will not be called.\nDrag off pins to build functionality.
)

(event EventOnExiting
  (params (isHappy :type Boolean) (is%20puta :type Boolean))
  (if (not is%20puta)
    (bind _asbp_gm_gameplay (Utilities|Casting|CastToBP_GM_Gameplay (Game|GetGameMode)))
    (Default|SetDialog (Variables|/Game/Marco/BP_GM_Gameplay.BP_GM_Gameplay_C|GetDialogue _asbp_gm_gameplay) "NewEnumerator1")))

(event EventOnGettingCommand
  (bind _asbp_gm_gameplay (Utilities|Casting|CastToBP_GM_Gameplay (Game|GetGameMode)))
  (Default|SetDialog (Variables|/Game/Marco/BP_GM_Gameplay.BP_GM_Gameplay_C|GetDialogue _asbp_gm_gameplay) "NewEnumerator0"))

(fn ConstructionScript
  (|CallParentFunction))
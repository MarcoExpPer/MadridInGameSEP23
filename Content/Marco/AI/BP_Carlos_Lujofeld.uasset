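; BP_Carlos_Lujofeld is a character-specific child Blueprint in the AI folder that triggers dialogue for Carlos Lujofeld.
; It sets one dialogue entry when getting a command and another when exiting unhappy; a happy exit triggers nothing.
; Both events reach the Dialogue object through BP_GM_Gameplay, and construction defers to the parent.
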(event EventOnExiting
  (params (isHappy :type Boolean) (is%20puta :type Boolean))
  (if (not isHappy)
    (bind _asbp_gm_gameplay (Utilities|Casting|CastToBP_GM_Gameplay (Game|GetGameMode)))
    (Default|SetDialog (Variables|/Game/Marco/BP_GM_Gameplay.BP_GM_Gameplay_C|GetDialogue _asbp_gm_gameplay) "NewEnumerator3")))

(event EventOnGettingCommand
  (bind _asbp_gm_gameplay (Utilities|Casting|CastToBP_GM_Gameplay (Game|GetGameMode)))
  (Default|SetDialog (Variables|/Game/Marco/BP_GM_Gameplay.BP_GM_Gameplay_C|GetDialogue _asbp_gm_gameplay) "NewEnumerator2"))

(fn ConstructionScript
  (|CallParentFunction))
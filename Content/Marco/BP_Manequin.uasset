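; BP_Manequin is a mannequin hazard that topples when StartFalling is called and stuns players.
; Tick interpolates its rotation toward TargetRotation; on arrival it stuns every BP_Player within a 2D radius and plays a sound.
; After a short delay it flags itself as on the floor and switches Cube collision to overlap on all channels.
; Cube overlaps with components tagged PlayerBody also stun that player.
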(event OnComponentBeginOverlap(Cube)
  (params (OverlappedComponent :type Primitive%20Component%20Object%20Reference) (OtherActor :type Actor%20Object%20Reference) (OtherComp :type Primitive%20Component%20Object%20Reference) (OtherBodyIndex :type Integer) (bFromSweep :type Boolean) (SweepResult :type Hit%20Result%20Structure%20%28by%20ref%29))
  (if (Components|ComponentHasTag OtherComp "PlayerBody")
    (bind _asbp_player (Utilities|Casting|CastToBP_Player OtherActor))
    (Default|HitbyStun _asbp_player)))

(event Custom|StartFalling
  (Variables|Default|SetcanBeActivated false)
  (Variables|Default|SetStartAnimation true))

(event EventBeginPlay)

(event Collision|EventActorBeginOverlap
  (params (OtherActor :type Actor%20Object%20Reference)))

(event EventTick
  (params (DeltaSeconds :type Float%20%28single-precision%29))
  (if (Variables|Default|GetStartAnimation)
    (Transformation|SetActorRotation (Math|Interpolation|RInterpTo (Transformation|GetActorRotation) (Variables|Default|GettargetRotation) DeltaSeconds 5.0))
    (if (Utilities|Operators|EqualEqual (Transformation|GetActorRotation) (Variables|Default|GettargetRotation) 0.5)
      (Variables|Default|SetStartAnimation false)
      (Transformation|SetActorRotation (Variables|Default|GettargetRotation))
      (bind _outactors (Actor|GetAllActorsOfClass "/Game/Marco/Player/BP_Player.BP_Player_C"))
      (for _array_element _outactors
        (if (<= (Math|Vector|Distance2D(Vector) (Transformation|GetActorLocation _array_element) (Transformation|GetWorldLocation (Variables|Default|GetScene))) 3.5e+02)
          (Default|HitbyStun _array_element)))
      (Audio|PlaySound2D "/Game/Audio/MS_Manniqui.MS_Manniqui" 1.0 1.0 0.0 0 0)
      (Utilities|FlowControl|Delay 1.0)
      (Variables|Default|SetisOnTheFloor true)
      (Collision|SetCollisionResponsetoAllChannels (Variables|Default|GetCube) "ECR_Overlap"))))

(fn ConstructionScript)
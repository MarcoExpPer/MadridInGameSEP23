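; Single-player game mode that clears the two-player flag on BeginPlay and is meant to ramp up client spawning as the match timer counts down.
; Tick checks descending CurrentTimer thresholds, each using a DoOnce to restart the Spawner with a shorter spawn interval.
; The checks chain through their false branches, so only the first threshold can fire and the faster stages are unreachable.
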(event EventBeginPlay
  (|CallParentFunction)
  (Variables|Default|SetisA2PlayerGame? false))

(event EventTick
  (params (DeltaSeconds :type Float%20%28single-precision%29))
  (|CallParentFunction DeltaSeconds)
  (if (<= (Variables|Default|GetcurrentTimer) 2.4e+02)
    (Utilities|FlowControl|DoOnce false
      (:Completed
        (Default|StartSpawningClients (Variables|Default|GetSpawner) 15.0 false)))
    (elif (<= (Variables|Default|GetcurrentTimer) 2e+02)
      (Utilities|FlowControl|DoOnce false
        (:Completed
          (Default|StartSpawningClients (Variables|Default|GetSpawner) 12.0 false)))
      (elif (<= (Variables|Default|GetcurrentTimer) 1.6e+02)
        (Utilities|FlowControl|DoOnce false
          (:Completed
            (Default|StartSpawningClients (Variables|Default|GetSpawner) 9.0 false)))
        (elif (<= (Variables|Default|GetcurrentTimer) 1.2e+02)
          (Utilities|FlowControl|DoOnce false
            (:Completed
              (Default|StartSpawningClients (Variables|Default|GetSpawner) 7.0 false)))
          (elif (<= (Variables|Default|GetcurrentTimer) 8e+01)
            (Utilities|FlowControl|DoOnce false
              (:Completed
                (Default|StartSpawningClients (Variables|Default|GetSpawner) 5.0 false)))))))))

(fn ConstructionScript
  (|CallParentFunction))
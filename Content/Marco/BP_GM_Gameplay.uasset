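; Gameplay game mode that runs a timed customer-serving level, from HUD setup to the results screen.
; BossFinished starts the countdown and client spawner after a short delay, and Tick drives the timer widget.
; Click events form a flag-gated tutorial, moving exclamation markers from counter desk through material, sewing and tint stations to exit counter.
; At timeout, FinishGame disables players, animates score progress with a Timeline, then opens GameOver.
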(event Custom|AddCustomerToQueue
  (params (NewItem :type BP%20Clientes%20Pj%20Object%20Reference%20%28by%20ref%29))
  (Utilities|Array|Add (Variables|Default|GetCustomerWaitList) NewItem))

(event Custom|StartLevel
  (params (maxTime :type Float%20%28double-precision%29))
  (Variables|Default|SetcurrentTimer (Variables|Rules|GetmaxTimer))
  (Variables|Default|SetinGame false))

(event Custom|BossFinished
  (Utilities|FlowControl|Delay 2.0)
  (Variables|Default|SetinGame true)
  (Default|StartSpawningClients (Variables|Default|GetSpawner) (Variables|Default|GetinitialClientSpawnTimer) true))

(event Custom|TogglePause
  (params (activate? :type Boolean))
  (Variables|Default|SetinGame (not activate?)))

(event Custom|Finish%20Game
  (Widget|RemovefromParent (Variables|Default|GetDialogue))
  (Widget|RemovefromParent (Variables|Default|GetWG_timer))
  (Input|SetInputModeUIOnly (Game|GetPlayerController 0) 0 "DoNotLock" false)
  (bind _outactors (Actor|GetAllActorsOfClass "/Game/Marco/Player/BP_Player.BP_Player_C"))
  (for _array_element _outactors
    (Default|DisableMovement _array_element))
  (Game|SetGamePaused false)
  (bind _returnvalue (UserInterface|CreateWidget "/Game/Marco/HUD/BPs/WG_LevelFinished.WG_LevelFinished_C"))
  (bind _output_get (Variables|Default|SetNewVar _returnvalue))
  (Default|UpdateProgress _output_get 0.0)
  (Default|UpdateText (Variables|Default|GetNewVar))
  (UserInterface|Viewport|AddtoViewport _output_get 0)
  (Variables|Default|SetisGameFinished? true)
  (Variables|Default|SetcurrentTimer 0.0)
  (bind _newtrack_0 (Timeline|Timeline PlayFromStart)
    (:Update
      (Default|UpdateProgress (Variables|Default|GetNewVar) (* (/ (Variables|Rules|GetinitialScore) (Variables|Rules|GetmaxManiqueScore)) _newtrack_0)))
    (:Finished
      (Default|UpdateText (Variables|Default|GetNewVar) (Utilities|Text|ToText(String) (Utilities|String|MakeLiteralString (Utilities|String|Append "Points: " (Utilities|String|MakeLiteralString (Utilities|String|ToString(Integer) (Math|Float|Truncate (Math|Float|Max(Float) (Variables|Rules|GetinitialScore) 0.0))))))))
      (Utilities|FlowControl|Delay (Variables|Rules|GetdelayToSeeScore))
      (Game|OpenLevel(byObjectReference) "/Game/Maps/GameOver.GameOver"))))

(event Custom|RemoveCustomerFromQueue
  (bind _customerwaitlist (Variables|Default|GetCustomerWaitList))
  (Development|PrintString (Utilities|String|ToString(Integer) (Utilities|Array|Length _customerwaitlist)))
  (Utilities|Array|RemoveIndex _customerwaitlist)
  (Development|PrintString (Utilities|String|ToString(Integer) (Utilities|Array|Length (Variables|Default|GetCustomerWaitList)))))

(event Custom|InitDeskClicked
  (if (not (Variables|Default|GethasClicked_InitDesk?))
    (Variables|Default|SethasClicked_InitDesk? true)
    (bind _outactors (Actor|GetAllActorsOfClass "/Game/Marco/Interactuables/BP_CounterDesk.BP_CounterDesk_C"))
    (for _array_element _outactors
      (Default|ToggleExclamation _array_element false))
    (bind _outactors_2 (Actor|GetAllActorsOfClass "/Game/Marco/Interactuables/BP_BaseMaterialGenerator.BP_BaseMaterialGenerator_C"))
    (for _array_element_2 _outactors_2
      (Default|ToggleExclamation _array_element_2 true))))

(event Custom|rawClicked
  (if (not (or (Variables|Default|GethasClicked_Raw?) (not (Variables|Default|GethasClicked_InitDesk?))))
    (Variables|Default|SethasClicked_Raw? true)
    (bind _outactors (Actor|GetAllActorsOfClass "/Game/Marco/Interactuables/BP_BaseMaterialGenerator.BP_BaseMaterialGenerator_C"))
    (for _array_element _outactors
      (Default|ToggleExclamation _array_element false))
    (bind _outactors_2 (Actor|GetAllActorsOfClass "/Game/Marco/Interactuables/BP_sewMachine.BP_sewMachine_C"))
    (for _array_element_2 _outactors_2
      (Default|ToggleExclamation _array_element_2 true))))

(event Custom|TintClicked
  (if (not (Math|Boolean|ORBoolean (Variables|Default|GethasClicked_Tint?) (not (Variables|Default|GethasClicked_InitDesk?)) (not (Variables|Default|GethasClicked_Raw?)) (not (Variables|Default|GethasClicked_Sew?))))
    (Variables|Default|SethasClicked_Tint? true)
    (bind _outactors (Actor|GetAllActorsOfClass "/Game/Marco/Interactuables/BP_TintMachine.BP_TintMachine_C"))
    (for _array_element _outactors
      (Default|ToggleExclamation _array_element false))
    (bind _outactors_2 (Actor|GetAllActorsOfClass "/Game/Marco/Interactuables/BP_CounterExit.BP_CounterExit_C"))
    (for _array_element_2 _outactors_2
      (Default|ToggleExclamation _array_element_2 true))))

(event Custom|sewClicked
  (if (not (Math|Boolean|ORBoolean (Variables|Default|GethasClicked_Tint?) (not (Variables|Default|GethasClicked_InitDesk?)) (not (Variables|Default|GethasClicked_Raw?))))
    (Variables|Default|SethasClicked_Sew? true)
    (bind _outactors (Actor|GetAllActorsOfClass "/Game/Marco/Interactuables/BP_sewMachine.BP_sewMachine_C"))
    (for _array_element _outactors
      (Default|ToggleExclamation _array_element false))
    (bind _outactors_2 (Actor|GetAllActorsOfClass "/Game/Marco/Interactuables/BP_TintMachine.BP_TintMachine_C"))
    (for _array_element_2 _outactors_2
      (Default|ToggleExclamation _array_element_2 true))))

(event Custom|endDeskClicked
  (if (not (Math|Boolean|ORBoolean (Variables|Default|GethasClicked_End?) (not (Variables|Default|GethasClicked_InitDesk?)) (not (Variables|Default|GethasClicked_Raw?)) (not (Variables|Default|GethasClicked_Sew?)) (not (Variables|Default|GethasClicked_Tint?))))
    (Variables|Default|SethasClicked_End? true)
    (bind _outactors (Actor|GetAllActorsOfClass "/Game/Marco/Interactuables/BP_CounterExit.BP_CounterExit_C"))
    (for _array_element _outactors
      (Default|ToggleExclamation _array_element false))))

(event EventBeginPlay
  (bind _returnvalue (UserInterface|CreateWidget "/Game/Deewa/UW_Gameplay.UW_Gameplay_C"))
  (bind _output_get (Variables|Default|SetWG_timer _returnvalue))
  (UserInterface|Viewport|AddtoViewport _returnvalue 0)
  (bind _returnvalue_2 (UserInterface|CreateWidget "/Game/Marco/HUD/Dialogs/WG_Dialog.WG_Dialog_C"))
  (bind _output_get_2 (Variables|Default|SetDialogue _returnvalue_2))
  (UserInterface|Viewport|AddtoViewport _output_get_2 0)
  (bind _returnvalue_3 (Actor|GetActorOfClass "/Game/Marco/AI/BP_Spawner.BP_Spawner_C"))
  (Variables|Default|SetSpawner _returnvalue_3))

(event EventTick
  (params (DeltaSeconds :type Float%20%28single-precision%29))
  (if (not (Variables|Default|GetisGameFinished?))
    (if (Variables|Default|GetinGame)
      (bind _output_get (Variables|Default|SetcurrentTimer (- (Variables|Default|GetcurrentTimer) DeltaSeconds)))
      (Default|UpdatePercentage (Variables|Default|GetWG_timer) (/ _output_get (Variables|Rules|GetmaxTimer)))
      (if (<= (Variables|Default|GetcurrentTimer) 0.0)
        (CallFunction|FinishGame)))))

(fn ConstructionScript)
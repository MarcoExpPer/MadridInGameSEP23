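; Two-player game mode variant that flags the match as two-player on BeginPlay and is meant to speed up client spawning as the timer counts down.
; Tick compares CurrentTimer against thresholds 40 seconds apart, each using a DoOnce to call the Spawner with a shorter spawn interval.
; Lower thresholds sit on the false branch of higher ones, so as wired only the first stage can fire.
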(event EventBeginPlay
  (|CallParentFunction)
  (Variables|Default|SetisA2PlayerGame? true))

(event EventTick
  (params (DeltaSeconds :type Float%20%28single-precision%29))
  (|CallParentFunction DeltaSeconds)
  (if (<= (Variables|Default|GetcurrentTimer) 2.6e+02)
    (Utilities|FlowControl|DoOnce false
      (:Completed
        (Default|StartSpawningClients (Variables|Default|GetSpawner) 11.0 false)))
    (elif (<= (Variables|Default|GetcurrentTimer) 2.2e+02)
      (Utilities|FlowControl|DoOnce false
        (:Completed
          (Default|StartSpawningClients (Variables|Default|GetSpawner) 9.0 false)))
      (elif (<= (Variables|Default|GetcurrentTimer) 1.8e+02)
        (Utilities|FlowControl|DoOnce false
          (:Completed
            (Default|StartSpawningClients (Variables|Default|GetSpawner) 7.0 false)))
        (elif (<= (Variables|Default|GetcurrentTimer) 1.4e+02)
          (Utilities|FlowControl|DoOnce false
            (:Completed
              (Default|StartSpawningClients (Variables|Default|GetSpawner) 5.0 false))))))))

(fn ConstructionScript
  (|CallParentFunction))
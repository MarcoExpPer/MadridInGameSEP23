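; Game mode for a two-player match that holds off starting the game until a second player joins.
; Each new player's name is printed, and a flag marks that the first has arrived.
; For any later player, it runs second-player setup on the BP_MultiPlayerCtrl, then after a short delay updates that controller's camera and tells the Spawner to start the game.
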(event EventBeginPlay
  (|CallParentFunction) ; This node is disabled and will not be called.\nDrag off pins to build functionality.
)

(event EventTick
  (params (DeltaSeconds :type Float%20%28single-precision%29))
  (|CallParentFunction DeltaSeconds) ; This node is disabled and will not be called.\nDrag off pins to build functionality.
)

(event EventHandleStartingNewPlayer
  (params (NewPlayer :type Player%20Controller%20Object%20Reference))
  (|CallParentFunction NewPlayer)
  (Development|PrintString (Utilities|GetDisplayName NewPlayer))
  (if (Variables|Default|GetisSecondPlayer?)
    (bind _asbp_multi_player_ctrl (Utilities|Casting|CastToBP_MultiPlayerCtrl NewPlayer))
    (Default|SecondPlayerSetup _asbp_multi_player_ctrl)
    (Utilities|FlowControl|Delay 0.2)
    (Default|UpdateCamera _asbp_multi_player_ctrl)
    (Default|StartGame (Variables|Default|GetSpawner))
    (else
      (Variables|Default|SetisSecondPlayer? true))))

(fn ConstructionScript
  (|CallParentFunction))
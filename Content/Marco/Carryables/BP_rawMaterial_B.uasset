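; Raw material "B" carryable, a child Blueprint that marks its variant by color.
; On BeginPlay it runs the parent logic, then sets the ColorTint parameter on the Cube's materials to red.
; It adds no other active logic: overlap and tick events are disabled stubs, and the construction script only calls the parent.
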(event EventBeginPlay
  (|CallParentFunction)
  (Rendering|Material|SetVectorParameterValueonMaterials (Variables|Default|GetCube) "ColorTint" (Math|Conversions|ToVector(LinearColor) (Utilities|Struct|MakeLinearColor 1.0 0.0 0.0 0.0))))

(event Collision|EventActorBeginOverlap
  (params (OtherActor :type Actor%20Object%20Reference))
  (|CallParentFunction OtherActor) ; This node is disabled and will not be called.\nDrag off pins to build functionality.
)

(event EventTick
  (params (DeltaSeconds :type Float%20%28single-precision%29))
  (|CallParentFunction DeltaSeconds) ; This node is disabled and will not be called.\nDrag off pins to build functionality.
)

(fn ConstructionScript
  (|CallParentFunction))
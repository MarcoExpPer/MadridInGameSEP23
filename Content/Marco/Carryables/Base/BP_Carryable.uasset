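; Base carryable item that starts raw, can be tinted and turned into a product, and moves between players and machines.
; ToProduct swaps the cube mesh to the left or right model from its Data, rescales the actor and reapplies any tint through the ColorTint material parameter.
; Snap events attach it to a player's CarryPoint, registering it as their Carryable, or to a machine's CarryablePoint.
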(event EventBeginPlay
  (Transformation|SetWorldScale3D (Variables|Default|GetCube) "0.500000,0.500000,0.250000"))

(event Collision|EventActorBeginOverlap
  (params (OtherActor :type Actor%20Object%20Reference)))

(event EventTick
  (params (DeltaSeconds :type Float%20%28single-precision%29)))

(event EventSnaptoPlayer
  (params (PlayerPawn :type BP%20Player%20Object%20Reference))
  (Transformation|AttachComponentToComponent (Variables|/Game/Marco/Player/BP_Player.BP_Player_C|GetCarryPoint PlayerPawn) "None" "SnapToTarget" "SnapToTarget" "KeepWorld" true)
  (Variables|/Game/Marco/Player/BP_Player.BP_Player_C|Setcarryable PlayerPawn self))

(event EventDespawn
  (Actor|DestroyActor))

(event EventSnaptoMachine
  (params (Interactuable :type BP%20Interactuable%20Object%20Reference))
  (Transformation|AttachComponentToComponent (Variables|/Game/Marco/Interactuables/Base/BP_Interactuable.BP_Interactuable_C|GetCarryablePoint Interactuable) "None" "SnapToTarget" "SnapToTarget" "KeepWorld" true))

(event EventToTint
  (params (tint :type Linear%20Color%20Structure))
  (Variables|Default|SetisTinted true)
  (bind _output_get (Variables|Default|SetcurrentTint tint))
  (Rendering|Material|SetVectorParameterValueonMaterials (Variables|Default|GetCube) "ColorTint" (Math|Conversions|ToVector(LinearColor) _output_get)))

(event EventToProduct
  (params (isLeftActivation :type Boolean))
  (bind _data (Variables|Default|Getdata))
  (bind _returnvalue (select isLeftActivation (.modelleft _data) (.modelright _data)))
  (Transformation|SetActorScale3D "6.000000,6.000000,6.000000")
  (Variables|Default|SetisLeftOption? isLeftActivation)
  (Development|PrintString (Utilities|GetDisplayName _returnvalue))
  (Components|StaticMesh|SetStaticMesh (Variables|Default|GetCube) _returnvalue)
  (Variables|Default|SetisRaw false)
  (if (Variables|Default|GetisTinted)
    (CallFunction|ToTint (Variables|Default|GetcurrentTint))))

(fn ConstructionScript)

(fn ObtainData
  (return (Variables|Default|Getdata)))
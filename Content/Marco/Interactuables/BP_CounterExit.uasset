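; BP_CounterExit is the delivery counter where the player hands a carried garment to the first waiting customer from BP_Spawner.
; Interact freezes the player, checks the item is tinted and not raw, then matches option, tint and raw class to the order.
; The three outcomes drive score, customer emotion and delayed sound, with some sounds muted during the tutorial.
; The item is then despawned, the customer leaves and movement returns.
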(event Custom|ReturnControlToPlayer
  (params (Target :type BP%20Player%20Object%20Reference))
  (Utilities|FlowControl|Delay 0.6)
  (Default|EnableMovement Target))

(event Custom|RemoveCarryable
  (params (player :type BP%20Player%20Object%20Reference))
  (Variables|/Game/Marco/Player/BP_Player.BP_Player_C|SetisCarrying player false)
  (Default|Despawn (Variables|/Game/Marco/Player/BP_Player.BP_Player_C|Getcarryable player))
  (Variables|/Game/Marco/Player/BP_Player.BP_Player_C|Setcarryable player 0)
  (Default|RemoveCustomerfromQueue (Variables|Default|GetBP_GM_Gameplay)))

(event Custom|ToggleExclamation
  (params (bNewVisibility :type Boolean))
  (Rendering|SetVisibility (Variables|Default|GetWidget) bNewVisibility false))

(event Custom|playSound
  (if (not (Variables|/Game/Marco/AI/BP_Spawner.BP_Spawner_C|GetinTutorial (Variables|Default|GetSpawner)))
    (Audio|PlaySound2D "/Game/Audio/Raw/entrega_prenda.entrega_prenda" 1.0 1.0 0.0 0 0)))

(event Custom|MalSound
  (if (not (Variables|/Game/Marco/AI/BP_Spawner.BP_Spawner_C|GetinTutorial (Variables|Default|GetSpawner)))
    (Audio|PlaySound2D "/Game/Audio/MS_Entrega_Mal.MS_Entrega_Mal" 1.0 1.0 0.0 0 0)))

(event Custom|IntermedioSOund
  (if (not (Variables|/Game/Marco/AI/BP_Spawner.BP_Spawner_C|GetinTutorial (Variables|Default|GetSpawner)))
    (Audio|PlaySound2D "/Game/Audio/MS_Entrega_Mid.MS_Entrega_Mid" 1.0 1.0 0.0 0 0)))

(event Custom|CorrectSound
  (Audio|PlaySound2D "/Game/Audio/MS_Entrega_Bien.MS_Entrega_Bien" 1.0 1.0 0.0 0 0))

(event EventBeginPlay
  (|CallParentFunction)
  (bind _asbp_gm_gameplay (Utilities|Casting|CastToBP_GM_Gameplay (Game|GetGameMode)))
  (Variables|Default|SetBP_GM_Gameplay _asbp_gm_gameplay)
  (bind _returnvalue (Actor|GetActorOfClass "/Game/Marco/AI/BP_Spawner.BP_Spawner_C"))
  (Variables|Default|SetSpawner _returnvalue))

(event Collision|EventActorBeginOverlap
  (params (OtherActor :type Actor%20Object%20Reference))
  (|CallParentFunction OtherActor) ; This node is disabled and will not be called.\nDrag off pins to build functionality.
)

(event EventTick
  (params (DeltaSeconds :type Float%20%28single-precision%29))
  (|CallParentFunction DeltaSeconds) ; This node is disabled and will not be called.\nDrag off pins to build functionality.
)

(event EventInteract
  (params (isCarrying :type Boolean) (playerInteracting :type BP%20Player%20Object%20Reference) (isLeftActivation? :type Boolean))
  (bind _spawner (Variables|Default|GetSpawner))
  (bind _spawner_2 (Variables|Default|GetSpawner))
  (bind _customersattheend (Variables|/Game/Marco/AI/BP_Spawner.BP_Spawner_C|GetcustomersAtTheEnd _spawner))
  (bind _customersattheend_2 (Variables|/Game/Marco/AI/BP_Spawner.BP_Spawner_C|GetcustomersAtTheEnd _spawner_2))
  (bind _output (Utilities|Array|Get(acopy) _customersattheend))
  (bind _output_2 (Utilities|Array|Get(acopy) _customersattheend_2))
  (Default|EndDeskClicked (Variables|Default|GetBP_GM_Gameplay))
  (if isCarrying
    (Default|DisableMovement playerInteracting)
    (Utilities|IsValid _output_2
      (:Is%20Valid
        (CallFunction|PlaySound)
        (bind _isvalid_ (CallFunction|CheckBaseConditions (Variables|/Game/Marco/Player/BP_Player.BP_Player_C|Getcarryable playerInteracting)))
        (if _isvalid_
          (bind _isvalid (CallFunction|CompareAdvancedConditions (Variables|/Game/Marco/Player/BP_Player.BP_Player_C|Getcarryable playerInteracting) _output_2))
          (if _isvalid
            (Math|Float|IncrementFloat (Variables|/Game/Marco/BP_GM_Gameplay.BP_GM_Gameplay_C|GetinitialScore (Variables|Default|GetBP_GM_Gameplay))
              (:%20%20
                (Default|ActivateEmotions _output true false)
                (Default|SendCustomerOutside (Variables|Default|GetSpawner) true)
                (CallFunction|ReturnControltoPlayer playerInteracting)
                (CallFunction|RemoveCarryable playerInteracting)
                (Utilities|Time|SetTimerbyEvent (delegate Custom|CorrectSound) 1.5)))
            (else
              (Default|ActivateEmotions _output false false)
              (Utilities|Time|SetTimerbyEvent (delegate Custom|IntermedioSOund) 1.5)
              (CallFunction|ReturnControltoPlayer playerInteracting :!label _label)
              (CallFunction|RemoveCarryable playerInteracting)
              (Default|SendCustomerOutside (Variables|Default|GetSpawner) false)))
          (else
            (Math|Float|DecrementFloat (Variables|/Game/Marco/BP_GM_Gameplay.BP_GM_Gameplay_C|GetinitialScore (Variables|Default|GetBP_GM_Gameplay))
              (:%20%20
                (Default|ActivateEmotions (Utilities|Array|Get(acopy) (Variables|/Game/Marco/AI/BP_Spawner.BP_Spawner_C|GetcustomersAtTheEnd (Variables|Default|GetSpawner))) false true)
                (Utilities|Time|SetTimerbyEvent (delegate Custom|MalSound) 1.5)
                (goto _label))))))
      (:Is%20Not%20Valid
        (Development|PrintString "NoOneToBuy")
        (CallFunction|ReturnControltoPlayer playerInteracting)))
    (else
      (Development|PrintString "Nothing to sell"))))

(fn ConstructionScript
  (|CallParentFunction))

(fn CheckBaseConditions
  (params (carryable :type BP%20Carryable%20Object%20Reference))
  (if (Variables|/Game/Marco/Carryables/Base/BP_Carryable.BP_Carryable_C|GetisTinted carryable)
    (if (Variables|/Game/Marco/Carryables/Base/BP_Carryable.BP_Carryable_C|GetisRaw carryable)
      (Development|PrintString "Is Raw!!")
      (return false)
      (else
        (Development|PrintString "Basic Characteristics are valid")
        (return true)))
    (else
      (Development|PrintString "No Tint!")
      (return false))))

(fn CompareAdvancedConditions
  (params (carryable :type BP%20Carryable%20Object%20Reference) (cust :type BP%20My%20Customer%20Object%20Reference))
  (if (== (Variables|/Game/Marco/Carryables/Base/BP_Carryable.BP_Carryable_C|GetisLeftOption? carryable) (Variables|/Game/Marco/AI/BP_MyCustomer.BP_MyCustomer_C|GetresultLeft cust))
    (if (== (Variables|/Game/Marco/Carryables/Base/BP_Carryable.BP_Carryable_C|GetcurrentTint carryable) (Variables|/Game/Marco/AI/BP_MyCustomer.BP_MyCustomer_C|GetresultTint cust))
      (if (== (.rawclass (Variables|/Game/Marco/Carryables/Base/BP_Carryable.BP_Carryable_C|Getdata carryable)) (.rawclass (Variables|/Game/Marco/AI/BP_MyCustomer.BP_MyCustomer_C|GetresultPattern cust)))
        (Development|PrintString "Everything is ok")
        (return true)
        (else
          (Development|PrintString "Not the same raw class")
          (return false)))
      (else
        (Development|PrintString "Not the same tint")
        (return false)))
    (else
      (Development|PrintString "Not left option")
      (return false))))
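; BP_FreeSpace is an interactable slot where a player sets down or picks up one carryable item.
; Its Interact event branches on whether the player is carrying and whether the slot is available.
; Placing snaps the item to this actor, while picking up snaps it back to the player, swapping Carryable references and flags both ways.
; Invalid attempts, such as an occupied slot or nothing to pick up, only print a debug string.
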(event EventBeginPlay
  (|CallParentFunction) ; This node is disabled and will not be called.\nDrag off pins to build functionality.
)

(event Collision|EventActorBeginOverlap
  (params (OtherActor :type Actor%20Object%20Reference))
  (|CallParentFunction OtherActor) ; This node is disabled and will not be called.\nDrag off pins to build functionality.
)

(event EventTick
  (params (DeltaSeconds :type Float%20%28single-precision%29))
  (|CallParentFunction DeltaSeconds) ; This node is disabled and will not be called.\nDrag off pins to build functionality.
)

(event EventInteract
  (params (isCarrying :type Boolean) (playerInteracting :type BP%20Player%20Object%20Reference) (isLeftActivation? :type Boolean))
  (if isCarrying
    (if (Variables|Default|GetisAvailable)
      (Variables|/Game/Marco/Player/BP_Player.BP_Player_C|SetisCarrying playerInteracting false)
      (Default|SnaptoMachine (Variables|/Game/Marco/Player/BP_Player.BP_Player_C|Getcarryable playerInteracting) self)
      (Variables|Default|Setcarryable (Variables|/Game/Marco/Player/BP_Player.BP_Player_C|Getcarryable playerInteracting))
      (Variables|/Game/Marco/Player/BP_Player.BP_Player_C|Setcarryable playerInteracting 0)
      (Variables|Default|SetisAvailable false)
      (else
        (Development|PrintString "FreeSpace already occupied")))
    (elif (Variables|Default|GetisAvailable)
      (Development|PrintString "Nothing to pick from Free Space")
      (else
        (Variables|/Game/Marco/Player/BP_Player.BP_Player_C|SetisCarrying playerInteracting true)
        (Default|SnaptoPlayer (Variables|Default|Getcarryable) playerInteracting)
        (Variables|/Game/Marco/Player/BP_Player.BP_Player_C|Setcarryable playerInteracting (Variables|Default|Getcarryable))
        (Variables|Default|Setcarryable 0)
        (Variables|Default|SetisAvailable true)))))

(fn ConstructionScript
  (|CallParentFunction))
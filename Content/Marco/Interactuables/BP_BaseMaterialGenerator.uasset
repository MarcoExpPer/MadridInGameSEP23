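; Base interactable generator that hands the player a raw material item to carry.
; On BeginPlay it briefly spawns a RawMaterial to read its data, destroys it, then shows that data's two sprites in the guide widget and hides the exclamation marker.
; Interact always notifies the gameplay GameMode, then, if the player's hands are free, spawns a material, snaps it to the player and plays a pickup sound.
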(event Custom|ToggleExclamation
  (params (newVisibility :type Boolean))
  (Rendering|SetVisibility (Variables|Default|GetExclamacionWidget) newVisibility false))

(event EventBeginPlay
  (|CallParentFunction)
  (bind _aswg_interactuable_guide_doube (Utilities|Casting|CastToWG_InteractuableGuideDoube (UserInterface|GetWidget (Variables|Default|GetGuideWidget))))
  (bind _output_get (Variables|Default|SetAs%20WG%20Interactuable%20Guide _aswg_interactuable_guide_doube))
  (Variables|/Script/UMG.Widget|SetRenderOpacity _output_get 0.0)
  (bind _returnvalue (Game|SpawnActorfromClass (Variables|Default|GetRawMaterial) (Transformation|GetActorTransform) "AlwaysSpawn" 0 0))
  (Variables|Default|SetRawMatData (Default|ObtainData _returnvalue))
  (Actor|DestroyActor _returnvalue)
  (CallFunction|ShowGuide)
  (CallFunction|ToggleExclamation false))

(event Collision|EventActorBeginOverlap
  (params (OtherActor :type Actor%20Object%20Reference))
  (|CallParentFunction OtherActor) ; This node is disabled and will not be called.\nDrag off pins to build functionality.
)

(event EventTick
  (params (DeltaSeconds :type Float%20%28single-precision%29))
  (|CallParentFunction DeltaSeconds) ; This node is disabled and will not be called.\nDrag off pins to build functionality.
)

(event EventInteract
  (params (isCarrying :type Boolean) (playerInteracting :type BP%20Player%20Object%20Reference) (isLeftActivation? :type Boolean))
  (bind _asbp_gm_gameplay (Utilities|Casting|CastToBP_GM_Gameplay (Game|GetGameMode)))
  (Default|RawClicked _asbp_gm_gameplay)
  (if (not isCarrying)
    (Variables|/Game/Marco/Player/BP_Player.BP_Player_C|SetisCarrying playerInteracting true)
    (bind _returnvalue (Game|SpawnActorfromClass (Variables|Default|GetRawMaterial) (Transformation|GetActorTransform) "AlwaysSpawn" 0 0))
    (Default|SnaptoPlayer _returnvalue playerInteracting)
    (Audio|PlaySound2D "/Game/Audio/MS_TakeCloth.MS_TakeCloth" 1.0 1.0 0.0 0 0)))

(event EventShowGuide
  (params (carrileable :type BP%20Carryable%20Object%20Reference))
  (bind _rawmatdata (Variables|Default|GetRawMatData))
  (bind _as_wg_interactuable_guide (Variables|Default|GetAs%20WG%20Interactuable%20Guide))
  (Default|UpdateLeftContent _as_wg_interactuable_guide (.spriteleft _rawmatdata))
  (Default|UpdateRightContent _as_wg_interactuable_guide (.spriteright _rawmatdata))
  (Variables|/Script/UMG.Widget|SetRenderOpacity (Variables|Default|GetAs%20WG%20Interactuable%20Guide) 1.0))

(fn ConstructionScript
  (|CallParentFunction))
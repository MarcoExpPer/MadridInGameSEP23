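; BP_CounterDesk is an interactable counter desk that players use to call up the next waiting customer.
; On Interact it notifies BP_GM_Gameplay that the desk was clicked, then asks BP_Spawner to advance one customer from its waiting list, or prints a debug message if none wait.
; The interacting player's movement is disabled for a brief delay during this.
; A separate event toggles the visibility of its exclamation widget.
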(event Custom|ToggleExclamation
  (params (bNewVisibility :type Boolean))
  (Rendering|SetVisibility (Variables|Default|GetExclamationWidget) bNewVisibility false))

(event EventBeginPlay
  (|CallParentFunction) ; This node is disabled and will not be called.\nDrag off pins to build functionality.
)

(event Collision|EventActorBeginOverlap
  (params (OtherActor :type Actor%20Object%20Reference))
  (|CallParentFunction OtherActor) ; This node is disabled and will not be called.\nDrag off pins to build functionality.
)

(event EventTick
  (params (DeltaSeconds :type Float%20%28single-precision%29))
  (|CallParentFunction DeltaSeconds) ; This node is disabled and will not be called.\nDrag off pins to build functionality.
)

(event EventInteract
  (params (isCarrying :type Boolean) (playerInteracting :type BP%20Player%20Object%20Reference) (isLeftActivation? :type Boolean))
  (bind _asbp_gm_gameplay (Utilities|Casting|CastToBP_GM_Gameplay (Game|GetGameMode)))
  (Default|InitDeskClicked _asbp_gm_gameplay)
  (Default|DisableMovement playerInteracting)
  (bind _returnvalue (Actor|GetActorOfClass "/Game/Marco/AI/BP_Spawner.BP_Spawner_C"))
  (if (== (Utilities|Array|Length (Variables|/Game/Marco/AI/BP_Spawner.BP_Spawner_C|GetcustomersWaiting _returnvalue)) 0)
    (Development|PrintString "No customers ready")
    (else
      (Default|AdvanceOnefromWaiting _returnvalue)))
  (Utilities|FlowControl|Delay 0.6)
  (Default|EnableMovement playerInteracting))

(fn ConstructionScript
  (|CallParentFunction))
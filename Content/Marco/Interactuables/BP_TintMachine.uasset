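; BP_TintMachine is an interactable station that dyes a carried, untinted item one of two colors, chosen by left or right activation.
; Interact snaps the item in or hands it back to the player, notifying the gameplay GameMode and hiding the color guide widget.
; Chained timers apply the tint, then ruin an uncollected item to black, while Tick fills and then drains the progress bar.
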(event Custom|ItemToOkey
  (Default|ToTint (Variables|Default|Getcarryable) (Math|Color|SelectColor (Variables|Default|GetleftTint) (Variables|Default|GetrightTint) (Variables|Default|GetisLeftActivation)))
  (bind _returnvalue (Utilities|Time|SetTimerbyEvent (delegate Custom|ToRubbish) (Variables|Default|GetOffsetToDestroy)))
  (Variables|Default|Settimer _returnvalue)
  (Variables|Default|SetisGoingToWaste? true)
  (Variables|Default|SetcurrentTimer (Variables|Default|GetOffsetToDestroy)))

(event Custom|ToRubbish
  (Default|ToTint (Variables|Default|Getcarryable) "(R=0.000000,G=0.000000,B=0.000000,A=1.000000)")
  (Variables|Default|SetcurrentTimer 0.0)
  (Variables|/Script/UMG.Widget|SetRenderOpacity (Variables|Default|GetWG_ProgressBar) 0.0))

(event Custom|ToggleExclamation
  (params (newVisibility :type Boolean))
  (Rendering|SetVisibility (Variables|Default|GetExclamationWidget) newVisibility false))

(event Custom|PlaySound
  (params (colorTinTsound :type Boolean))
  (if colorTinTsound
    _
    (else
      _))
  (Utilities|IsValid (Variables|Default|GetblackSound)
    (:Is%20Valid
      (Audio|Components|Audio|Play (Variables|Default|GetblackSound) 0.0))
    (:Is%20Not%20Valid
      (bind _returnvalue (Audio|SpawnSound2D "/Game/Audio/Raw/teñir_completo_v3.teñir_completo_v3" 1.0 1.0 0.0 0))
      (Variables|Default|SetblackSound _returnvalue))))

(event Custom|stopAllSound
  (bind _blacksound (Variables|Default|GetblackSound))
  (bind _colorsound (Variables|Default|GetcolorSound))
  (Utilities|IsValid _colorsound
    (:Is%20Valid
      (Audio|Components|Audio|Stop _colorsound))
    (:Is%20Not%20Valid
      _))
  (Utilities|IsValid _blacksound
    (:Is%20Valid
      (Audio|Components|Audio|Stop _blacksound))))

(event EventBeginPlay
  (bind _aswg_progress_bar (Utilities|Casting|CastToWG_ProgressBar (UserInterface|GetWidget (Variables|Default|GetProgressBar))))
  (bind _output_get (Variables|Default|SetWG_ProgressBar _aswg_progress_bar))
  (Variables|/Script/UMG.Widget|SetRenderOpacity _output_get 0.0)
  (bind _aswg_interactuable_guide_tint (Utilities|Casting|CastToWG_InteractuableGuideTINT (UserInterface|GetWidget (Variables|Default|GetGuideWidget))))
  (bind _output_get_2 (Variables|Default|SetNewVar _aswg_interactuable_guide_tint))
  (Variables|/Script/UMG.Widget|SetRenderOpacity _output_get_2 0.0))

(event EventTick
  (params (DeltaSeconds :type Float%20%28single-precision%29))
  (if (not (Variables|Default|GetisAvailable))
    (if (Variables|Default|GetisGoingToWaste?)
      (bind _output_get (Variables|Default|SetcurrentTimer (- (Variables|Default|GetcurrentTimer) DeltaSeconds)))
      (Default|UpdatePercent (Variables|Default|GetWG_ProgressBar) (/ _output_get (Variables|Default|GetOffsetToDestroy)))
      (else
        (bind _output_get_2 (Variables|Default|SetcurrentTimer (+ (Variables|Default|GetcurrentTimer) DeltaSeconds)))
        (Default|UpdatePercent (Variables|Default|GetWG_ProgressBar) (/ _output_get_2 (Variables|Default|GettimeToOkey)))))))

(event EventInteract
  (params (isCarrying :type Boolean) (playerInteracting :type BP%20Player%20Object%20Reference) (isLeftActivation? :type Boolean))
  (bind _asbp_gm_gameplay (Utilities|Casting|CastToBP_GM_Gameplay (Game|GetGameMode)))
  (Default|TintClicked _asbp_gm_gameplay)
  (CallFunction|HideGuide)
  (if (Variables|Default|GetisAvailable)
    (if isCarrying
      (if (Variables|/Game/Marco/Carryables/Base/BP_Carryable.BP_Carryable_C|GetisTinted (Variables|/Game/Marco/Player/BP_Player.BP_Player_C|Getcarryable playerInteracting))
        (Development|PrintString "Already tinted")
        (else
          (Variables|Default|SetisLeftActivation isLeftActivation?)
          (Variables|/Game/Marco/Player/BP_Player.BP_Player_C|SetisCarrying playerInteracting false)
          (Default|SnaptoMachine (Variables|/Game/Marco/Player/BP_Player.BP_Player_C|Getcarryable playerInteracting) self)
          (Variables|Default|SetisAvailable false)
          (Variables|Default|Setcarryable (Variables|/Game/Marco/Player/BP_Player.BP_Player_C|Getcarryable playerInteracting))
          (Variables|/Game/Marco/Player/BP_Player.BP_Player_C|Setcarryable playerInteracting 0)
          (Utilities|Time|ClearandInvalidateTimerbyHandle (Variables|Default|Gettimer))
          (bind _returnvalue (Utilities|Time|SetTimerbyEvent (delegate Custom|ItemToOkey) (Variables|Default|GettimeToOkey)))
          (Variables|Default|Settimer _returnvalue)
          (Variables|Default|SetcurrentTimer 0.0)
          (Variables|Default|SetisGoingToWaste? false)
          (Variables|/Script/UMG.Widget|SetRenderOpacity (Variables|Default|GetWG_ProgressBar) 1.0)
          (CallFunction|PlaySound true)))
      (else
        (Development|PrintString "Nothing to tint")))
    (elif isCarrying
      (Development|PrintString "Cant Carry More")
      (else
        (Utilities|Time|ClearandInvalidateTimerbyHandle (Variables|Default|Gettimer))
        (Variables|/Game/Marco/Player/BP_Player.BP_Player_C|SetisCarrying playerInteracting true)
        (Variables|/Game/Marco/Player/BP_Player.BP_Player_C|Setcarryable playerInteracting (Variables|Default|Getcarryable))
        (Default|SnaptoPlayer (Variables|Default|Getcarryable) playerInteracting)
        (Variables|Default|Setcarryable 0)
        (Variables|Default|SetisAvailable true)
        (Variables|Default|SetcurrentTimer 0.0)
        (Variables|/Script/UMG.Widget|SetRenderOpacity (Variables|Default|GetWG_ProgressBar) 0.0)
        (CallFunction|StopAllSound)))))

(event EventShowGuide
  (params (carrileable :type BP%20Carryable%20Object%20Reference))
  (if (Variables|Default|GetisAvailable)
    (Default|UpdateLeftColor (Variables|Default|GetNewVar) (Variables|Default|GetleftTint))
    (Default|UpdateRightColor (Variables|Default|GetNewVar) (Variables|Default|GetrightTint))
    (Variables|/Script/UMG.Widget|SetRenderOpacity (Variables|Default|GetNewVar) 1.0)))

(event EventHideGuide
  (Variables|/Script/UMG.Widget|SetRenderOpacity (Variables|Default|GetNewVar) 0.0))

(fn ConstructionScript
  (|CallParentFunction))
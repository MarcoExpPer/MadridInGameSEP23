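; Sewing machine interactable that turns a player's carried raw cloth into a product, with left or right activation passed on to choose the result.
; Interact snaps the cloth to the machine, locks the player's movement and starts a timer, while Tick fills a progress bar widget.
; On completion, or when the engaged player interacts again to cancel, the item returns and movement resumes.
; A guide widget previews both options from the cloth's data.
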(event Custom|SewFinished
  (Default|ToProduct (Variables|Default|Getcarryable) (Variables|Default|GetisLeftActivation?))
  (CallFunction|ReturnCarryabletoPlayer (Variables|Default|GetengagedPlayer))
  (Variables|Default|SetcurrentTimer 0.0)
  (Variables|/Script/UMG.Widget|SetRenderOpacity (Variables|Default|GetAs%20WG%20Progress%20Bar) 0.0))

(event Custom|ToggleExclamation
  (params (newVisibility :type Boolean))
  (Rendering|SetVisibility (Variables|Default|GetExclamationWidget) newVisibility false))

(event EventBeginPlay
  (bind _aswg_progress_bar (Utilities|Casting|CastToWG_ProgressBar (UserInterface|GetWidget (Variables|Default|GetProgressBar))))
  (bind _output_get (Variables|Default|SetAs%20WG%20Progress%20Bar _aswg_progress_bar))
  (Variables|/Script/UMG.Widget|SetRenderOpacity _output_get 0.0)
  (bind _aswg_interactuable_guide (Utilities|Casting|CastToWG_InteractuableGuide (UserInterface|GetWidget (Variables|Default|GetGuide))))
  (Variables|Default|SetguideWG _aswg_interactuable_guide)
  (Variables|/Script/UMG.Widget|SetRenderOpacity _aswg_interactuable_guide 0.0))

(event EventTick
  (params (DeltaSeconds :type Float%20%28single-precision%29))
  (if (not (Variables|Default|GetisAvailable))
    (bind _output_get (Variables|Default|SetcurrentTimer (+ (Variables|Default|GetcurrentTimer) DeltaSeconds)))
    (Default|UpdatePercent (Variables|Default|GetAs%20WG%20Progress%20Bar) (/ _output_get (Variables|Default|GettimeToFinishSew)))))

(event EventInteract
  (params (isCarrying :type Boolean) (playerInteracting :type BP%20Player%20Object%20Reference) (isLeftActivation? :type Boolean))
  (bind _as_wg_progress_bar (Variables|Default|GetAs%20WG%20Progress%20Bar))
  (bind _asbp_gm_gameplay (Utilities|Casting|CastToBP_GM_Gameplay (Game|GetGameMode)))
  (Default|SewClicked _asbp_gm_gameplay)
  (CallFunction|HideGuide)
  (if (Variables|Default|GetisAvailable)
    (if isCarrying
      (if (Variables|/Game/Marco/Carryables/Base/BP_Carryable.BP_Carryable_C|GetisRaw (Variables|/Game/Marco/Player/BP_Player.BP_Player_C|Getcarryable playerInteracting))
        (Variables|Default|SetisLeftActivation? isLeftActivation?)
        (Variables|/Game/Marco/Player/BP_Player.BP_Player_C|SetisCarrying playerInteracting false)
        (bind _output_get (Variables|Default|Setcarryable (Variables|/Game/Marco/Player/BP_Player.BP_Player_C|Getcarryable playerInteracting)))
        (Default|SnaptoMachine _output_get self)
        (Variables|/Game/Marco/Player/BP_Player.BP_Player_C|Setcarryable playerInteracting 0)
        (Default|DisableMovement playerInteracting)
        (Variables|Default|SetengagedPlayer playerInteracting)
        (Variables|Default|SetisAvailable false)
        (Utilities|Time|ClearandInvalidateTimerbyHandle (Variables|Default|GetsewTimer))
        (bind _returnvalue (Utilities|Time|SetTimerbyEvent (delegate Custom|SewFinished) (Variables|Default|GettimeToFinishSew)))
        (Variables|Default|SetsewTimer _returnvalue)
        (Default|UpdatePercent _as_wg_progress_bar 0.0)
        (Variables|/Script/UMG.Widget|SetRenderOpacity _as_wg_progress_bar 1.0)
        (Variables|Default|SetcurrentTimer 0.0)
        (Utilities|IsValid (Variables|Default|GetCoserSound)
          (:Is%20Valid
            (Audio|Components|Audio|Play (Variables|Default|GetCoserSound) 0.0))
          (:Is%20Not%20Valid
            (bind _returnvalue_2 (Audio|SpawnSound2D "/Game/Audio/Raw/coser.coser" 1.0 1.0 0.0 0))
            (Variables|Default|SetCoserSound _returnvalue_2)))
        (else
          (Development|PrintString "Is not a raw cloth")))
      (else
        (Development|PrintString "Nothing to sew")))
    (elif (== playerInteracting (Variables|Default|GetengagedPlayer))
      (CallFunction|ReturnCarryabletoPlayer playerInteracting)
      (Variables|/Script/UMG.Widget|SetRenderOpacity (Variables|Default|GetAs%20WG%20Progress%20Bar) 0.0)
      (Audio|Components|Audio|Stop (Variables|Default|GetCoserSound))
      (else
        (Development|PrintString "Another player is already sewing")))))

(event EventShowGuide
  (params (carrileable :type BP%20Carryable%20Object%20Reference))
  (bind _data (Variables|/Game/Marco/Carryables/Base/BP_Carryable.BP_Carryable_C|Getdata carrileable))
  (bind _guidewg (Variables|Default|GetguideWG))
  (Utilities|IsValid carrileable
    (:Is%20Valid
      (Default|UpdateLeftContent (Variables|Default|GetguideWG) (.spriteleft _data))
      (Default|UpdateRightContent _guidewg (.spriteright _data))
      (Variables|/Script/UMG.Widget|SetRenderOpacity _guidewg 1.0))))

(event EventHideGuide
  (Variables|/Script/UMG.Widget|SetRenderOpacity (Variables|Default|GetguideWG) 0.0))

(fn ConstructionScript
  (|CallParentFunction))

(fn ReturnCarryabletoPlayer
  (params (player :type BP%20Player%20Object%20Reference))
  (Variables|/Game/Marco/Player/BP_Player.BP_Player_C|SetisCarrying player true)
  (Default|SnaptoPlayer (Variables|Default|Getcarryable) player)
  (Default|EnableMovement player)
  (Variables|/Game/Marco/Player/BP_Player.BP_Player_C|Setcarryable player (Variables|Default|Getcarryable))
  (Variables|Default|Setcarryable 0)
  (Variables|Default|SetisAvailable true)
  (Variables|Default|SetengagedPlayer 0)
  (Utilities|Time|ClearandInvalidateTimerbyHandle (Variables|Default|GetsewTimer)))
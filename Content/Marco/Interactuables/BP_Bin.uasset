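; BP_Bin is an interactable trash bin that lets a player discard the item they are carrying.
; On Interact, if the player is carrying, it clears their carry flag, despawns the Carryable, clears the reference and plays the Basura 2D sound.
; Interacting empty-handed does nothing, as the "Nothing to trash" debug print is never run.
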(event EventBeginPlay
  (|CallParentFunction) ; This node is disabled and will not be called.\nDrag off pins to build functionality.
)

(event Collision|EventActorBeginOverlap
  (params (OtherActor :type Actor%20Object%20Reference))
  (|CallParentFunction OtherActor) ; This node is disabled and will not be called.\nDrag off pins to build functionality.
)

(event EventTick
  (params (DeltaSeconds :type Float%20%28single-precision%29))
  (|CallParentFunction DeltaSeconds) ; This node is disabled and will not be called.\nDrag off pins to build functionality.
)

(event EventInteract
  (params (isCarrying :type Boolean) (playerInteracting :type BP%20Player%20Object%20Reference) (isLeftActivation? :type Boolean))
  (if isCarrying
    (Variables|/Game/Marco/Player/BP_Player.BP_Player_C|SetisCarrying playerInteracting false)
    (Default|Despawn (Variables|/Game/Marco/Player/BP_Player.BP_Player_C|Getcarryable playerInteracting))
    (Variables|/Game/Marco/Player/BP_Player.BP_Player_C|Setcarryable playerInteracting 0)
    (Audio|PlaySound2D "/Game/Audio/Raw/basura.basura" 1.0 1.0 0.0 0 0)))

(fn ConstructionScript
  (|CallParentFunction))
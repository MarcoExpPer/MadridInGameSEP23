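; Player controller that drives two BP_Player characters from one controller, for either solo character swapping or local two-player play.
; BeginPlay adds the input mapping, then retries until it finds the second character and game mode, restyling that character.
; Primary inputs route to the active character, swappable outside two-player mode with arrow indicators, while duplicate "_2" inputs target Player2 behind a check.
; It also toggles the pause menu, notifying the game mode.
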(event Custom|EndPause
  (bind _wg_pause (Variables|Default|GetWG_pause))
  (Utilities|IsValid _wg_pause
    (:Is%20Valid
      (Widget|RemovefromParent _wg_pause)
      (Variables|Default|SetbShowMouseCursor false)
      (Game|SetGamePaused false)
      (bind _asbp_gm_gameplay (Utilities|Casting|CastToBP_GM_Gameplay (Game|GetGameMode)))
      (Default|TogglePause _asbp_gm_gameplay false))))

(event Input|EnhancedActionEvents|EnhancedInputActionI_ActionA
  (params (ActionValue :type Boolean) (ElapsedSeconds :type Float%20%28double-precision%29) (TriggeredSeconds :type Float%20%28double-precision%29) (InputAction :type Input%20Action%20Object%20Reference :default "/Game/Marco/Player/Input/I_ActionA.I_ActionA"))
  ;[1 1 1] ACTION A
  (:Started
    (Default|ActionA (select (Variables|Default|GetisPlayer1TheCurrentActivePlayer) (Variables|Default|Getplayer_1) (Variables|Default|Getplayer_2)))))

(event Input|EnhancedActionEvents|EnhancedInputActionI_ActionA_2
  (params (ActionValue :type Boolean) (ElapsedSeconds :type Float%20%28double-precision%29) (TriggeredSeconds :type Float%20%28double-precision%29) (InputAction :type Input%20Action%20Object%20Reference :default "/Game/Marco/Player/Input/I_ActionA_2.I_ActionA_2"))
  ;[1 1 1] ACTION A
  (:Started
    (if (Utilities|Can2PlayerInputbeUsed?)
      (Default|ActionA (Variables|Default|Getplayer_2)))))

(event Input|EnhancedActionEvents|EnhancedInputActionI_ActionB_2
  (params (ActionValue :type Boolean) (ElapsedSeconds :type Float%20%28double-precision%29) (TriggeredSeconds :type Float%20%28double-precision%29) (InputAction :type Input%20Action%20Object%20Reference :default "/Game/Marco/Player/Input/I_ActionB_2.I_ActionB_2"))
  ;[1 1 1] Action B
  (:Started
    (if (Utilities|Can2PlayerInputbeUsed?)
      (Default|ActionB (Variables|Default|Getplayer_2)))))

(event Input|EnhancedActionEvents|EnhancedInputActionI_ActionB
  (params (ActionValue :type Boolean) (ElapsedSeconds :type Float%20%28double-precision%29) (TriggeredSeconds :type Float%20%28double-precision%29) (InputAction :type Input%20Action%20Object%20Reference :default "/Game/Marco/Player/Input/I_ActionB.I_ActionB"))
  ;[1 1 1] Action B
  (:Started
    (Default|ActionB (select (Variables|Default|GetisPlayer1TheCurrentActivePlayer) (Variables|Default|Getplayer_1) (Variables|Default|Getplayer_2)))))

(event Input|EnhancedActionEvents|EnhancedInputActionI_MoveRight
  (params (ActionValue :type Float%20%28double-precision%29) (ElapsedSeconds :type Float%20%28double-precision%29) (TriggeredSeconds :type Float%20%28double-precision%29) (InputAction :type Input%20Action%20Object%20Reference :default "/Game/Marco/Player/Input/I_MoveRight.I_MoveRight"))
  ;[1 1 1] MOVE RIGHT
  (:Triggered
    (Default|MoveRight (select (Variables|Default|GetisPlayer1TheCurrentActivePlayer) (Variables|Default|Getplayer_1) (Variables|Default|Getplayer_2)) ActionValue)))

(event Input|EnhancedActionEvents|EnhancedInputActionI_MoveRight_2
  (params (ActionValue :type Float%20%28double-precision%29) (ElapsedSeconds :type Float%20%28double-precision%29) (TriggeredSeconds :type Float%20%28double-precision%29) (InputAction :type Input%20Action%20Object%20Reference :default "/Game/Marco/Player/Input/I_MoveRight_2.I_MoveRight_2"))
  ;[1 1 1] MOVE RIGHT
  (:Triggered
    (if (Utilities|Can2PlayerInputbeUsed?)
      (Default|MoveRight (Variables|Default|Getplayer_2) ActionValue))))

(event Input|EnhancedActionEvents|EnhancedInputActionI_MoveUp
  (params (ActionValue :type Float%20%28double-precision%29) (ElapsedSeconds :type Float%20%28double-precision%29) (TriggeredSeconds :type Float%20%28double-precision%29) (InputAction :type Input%20Action%20Object%20Reference :default "/Game/Marco/Player/Input/I_MoveUp.I_MoveUp"))
  ;[1 1 1] MOVE UP
  (:Triggered
    (Default|MoveUp (select (Variables|Default|GetisPlayer1TheCurrentActivePlayer) (Variables|Default|Getplayer_1) (Variables|Default|Getplayer_2)) ActionValue)))

(event Input|EnhancedActionEvents|EnhancedInputActionI_MoveUp_2
  (params (ActionValue :type Float%20%28double-precision%29) (ElapsedSeconds :type Float%20%28double-precision%29) (TriggeredSeconds :type Float%20%28double-precision%29) (InputAction :type Input%20Action%20Object%20Reference :default "/Game/Marco/Player/Input/I_MoveUp_2.I_MoveUp_2"))
  ;[1 1 1] MOVE UP
  (:Triggered
    (if (Utilities|Can2PlayerInputbeUsed?)
      (Default|MoveUp (Variables|Default|Getplayer_2) ActionValue))))

(event Input|EnhancedActionEvents|EnhancedInputActionI_Pause
  (params (ActionValue :type Boolean) (ElapsedSeconds :type Float%20%28double-precision%29) (TriggeredSeconds :type Float%20%28double-precision%29) (InputAction :type Input%20Action%20Object%20Reference :default "/Game/Marco/Player/Input/I_Pause.I_Pause"))
  (:Started
    (if (Game|IsGamePaused)
      (Utilities|IsValid (Variables|Default|GetWG_pause)
        (:Is%20Valid
          (Widget|RemovefromParent (Variables|Default|GetWG_pause))
          (Variables|Default|SetbShowMouseCursor false)
          (Game|SetGamePaused false)
          (bind _asbp_gm_gameplay (Utilities|Casting|CastToBP_GM_Gameplay (Game|GetGameMode)))
          (Default|TogglePause _asbp_gm_gameplay false)))
      (else
        (Utilities|IsValid (Variables|Default|GetWG_pause)
          (:Is%20Valid
            _)
          (:Is%20Not%20Valid
            (bind _returnvalue (UserInterface|CreateWidget "/Game/Marco/HUD/BPs/WG_PauseMenu.WG_PauseMenu_C"))
            (Variables|Default|SetWG_pause _returnvalue)))
        (UserInterface|Viewport|AddtoViewport (Variables|Default|GetWG_pause) 0)
        (Variables|Default|SetbShowMouseCursor true)
        (bind _asbp_gm_gameplay_2 (Utilities|Casting|CastToBP_GM_Gameplay (Game|GetGameMode)))
        (Default|TogglePause _asbp_gm_gameplay_2 true)
        (Game|SetGamePaused true)))))

(event Input|EnhancedActionEvents|EnhancedInputActionI_SwapCharacter
  (params (ActionValue :type Boolean) (ElapsedSeconds :type Float%20%28double-precision%29) (TriggeredSeconds :type Float%20%28double-precision%29) (InputAction :type Input%20Action%20Object%20Reference :default "/Game/Marco/Player/Input/I_SwapCharacter.I_SwapCharacter"))
  (:Started
    (if (Math|Boolean|ANDBoolean (Utilities|IsValid (Variables|Default|Getplayer_2)) (Utilities|IsValid (Variables|Default|GetGM)) (not (Variables|/Game/Marco/BP_GM_Gameplay.BP_GM_Gameplay_C|GetisA2PlayerGame? (Variables|Default|GetGM))))
      (Variables|Default|SetisPlayer1TheCurrentActivePlayer (not (Variables|Default|GetisPlayer1TheCurrentActivePlayer)))
      (Default|ToggleArrow (Variables|Default|Getplayer_1) (Variables|Default|GetisPlayer1TheCurrentActivePlayer))
      (Default|ToggleArrow (Variables|Default|Getplayer_2) (not (Variables|Default|GetisPlayer1TheCurrentActivePlayer))))))

(event EventBeginPlay
  (Input|AddMappingContext (PlayerController|LocalPlayerSubsystems|GetEnhancedInputLocalPlayerSubsystem self) "/Game/Marco/Player/Input/IM_Player.IM_Player" 0 "(bIgnoreAllPressedKeysUntilRelease=True,bForceImmediately=False)")
  (bind _asbp_player (Utilities|Casting|CastToBP_Player (Pawn|GetControlledPawn)))
  (Variables|Default|Setplayer_1 _asbp_player)
  (bind _asbp_gm_gameplay (Utilities|Casting|CastToBP_GM_Gameplay (Game|GetGameMode) :!label _label)
    (:then
      (Variables|Default|SetGM _asbp_gm_gameplay))
    (:CastFailed
      _))
  (bind _outactors (Actor|GetAllActorsOfClass "/Game/Marco/Player/BP_Player.BP_Player_C"))
  (bind _array_element (Utilities|Array|ForEachLoopwithBreak _outactors :!label _label_2)
    (:LoopBody
      (if (!= _array_element (Variables|Default|Getplayer_1))
        (Variables|Default|Setplayer_2 _array_element)
        (goto _label_2 Break)))
    (:Completed
      (if (and (Utilities|IsValid (Variables|Default|Getplayer_2)) (Utilities|IsValid (Variables|Default|GetGM)))
        (Components|SkeletalMesh|SetSkeletalMeshAsset (Variables|/Script/Engine.Character|GetMesh (Variables|Default|Getplayer_2)) "/Game/Deewa/animation/ClienteIdle.ClienteIdle")
        (Rendering|Material|SetMaterial (Variables|/Script/Engine.Character|GetMesh (Variables|Default|Getplayer_2)) 0 "/Game/Materials/MI_Oliva.MI_Oliva")
        (if (not (Variables|/Game/Marco/BP_GM_Gameplay.BP_GM_Gameplay_C|GetisA2PlayerGame? (Variables|Default|GetGM)))
          (Utilities|FlowControl|Delay 0.2)
          (Default|ToggleArrow (Variables|Default|Getplayer_1) true))
        (else
          (Utilities|FlowControl|Delay 0.2)
          (goto _label))))))

(fn ConstructionScript)
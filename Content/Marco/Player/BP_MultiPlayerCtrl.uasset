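; Player controller for local multiplayer that forwards Enhanced Input move and action presses to its cached BP_Player pawn.
; On BeginPlay it adds the multiplayer mapping context, caches the pawn and switches the view to a CameraActor in the level.
; SecondPlayerSetup flags the second player, reskinning its pawn with a different mesh and material.
; Pause input toggles the pause menu, cursor and game pause, notifying BP_GM_Gameplay.
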(event Custom|EndPause
  (bind _wg_pause (Variables|Default|GetWG_pause))
  (Utilities|IsValid _wg_pause
    (:Is%20Valid
      (Widget|RemovefromParent _wg_pause)
      (Variables|Default|SetbShowMouseCursor false)
      (Game|SetGamePaused false)
      (bind _asbp_gm_gameplay (Utilities|Casting|CastToBP_GM_Gameplay (Game|GetGameMode)))
      (Default|TogglePause _asbp_gm_gameplay false))))

(event Custom|CachePlayerPawn
  (Utilities|IsValid (Variables|Default|Getplayer_1)
    (:Is%20Valid
      _)
    (:Is%20Not%20Valid
      (bind _asbp_player (Utilities|Casting|CastToBP_Player (Pawn|GetControlledPawn)))
      (Variables|Default|Setplayer_1 _asbp_player)))
  (if (Variables|Default|GetisSecondPlayer)
    (Components|SkeletalMesh|SetSkeletalMeshAsset (Variables|/Script/Engine.Character|GetMesh (Variables|Default|Getplayer_1)) "/Game/Deewa/animation/ClienteIdle.ClienteIdle")
    (Rendering|Material|SetMaterial (Variables|/Script/Engine.Character|GetMesh (Variables|Default|Getplayer_1)) 0 "/Game/Materials/MI_Oliva.MI_Oliva")))

(event Custom|UpdateCamera
  (bind _returnvalue (Actor|GetActorOfClass "/Script/Engine.CameraActor"))
  (Development|PrintString (Utilities|GetDisplayName _returnvalue))
  (Game|Player|SetViewTargetwithBlend self _returnvalue 0.0 "VTBlend_Linear" 0.0 false))

(event Custom|SecondPlayerSetup
  (Development|PrintString (Utilities|GetDisplayName self))
  (Variables|Default|SetisSecondPlayer true)
  (CallFunction|CachePlayerPawn)
  (CallFunction|UpdateCamera))

(event Input|EnhancedActionEvents|EnhancedInputActionI_ActionA
  (params (ActionValue :type Boolean) (ElapsedSeconds :type Float%20%28double-precision%29) (TriggeredSeconds :type Float%20%28double-precision%29) (InputAction :type Input%20Action%20Object%20Reference :default "/Game/Marco/Player/Input/I_ActionA.I_ActionA"))
  ;[1 1 1] ACTION A
  (:Started
    (Default|ActionA (Variables|Default|Getplayer_1))))

(event Input|EnhancedActionEvents|EnhancedInputActionI_ActionB
  (params (ActionValue :type Boolean) (ElapsedSeconds :type Float%20%28double-precision%29) (TriggeredSeconds :type Float%20%28double-precision%29) (InputAction :type Input%20Action%20Object%20Reference :default "/Game/Marco/Player/Input/I_ActionB.I_ActionB"))
  ;[1 1 1] Action B
  (:Started
    (Default|ActionB (Variables|Default|Getplayer_1))))

(event Input|EnhancedActionEvents|EnhancedInputActionI_MoveRight
  (params (ActionValue :type Float%20%28double-precision%29) (ElapsedSeconds :type Float%20%28double-precision%29) (TriggeredSeconds :type Float%20%28double-precision%29) (InputAction :type Input%20Action%20Object%20Reference :default "/Game/Marco/Player/Input/I_MoveRight.I_MoveRight"))
  ;[1 1 1] MOVE RIGHT
  (:Triggered
    (Default|MoveRight (Variables|Default|Getplayer_1) ActionValue)))

(event Input|EnhancedActionEvents|EnhancedInputActionI_MoveUp
  (params (ActionValue :type Float%20%28double-precision%29) (ElapsedSeconds :type Float%20%28double-precision%29) (TriggeredSeconds :type Float%20%28double-precision%29) (InputAction :type Input%20Action%20Object%20Reference :default "/Game/Marco/Player/Input/I_MoveUp.I_MoveUp"))
  ;[1 1 1] MOVE UP
  (:Triggered
    (Default|MoveUp (Variables|Default|Getplayer_1) ActionValue)))

(event Input|EnhancedActionEvents|EnhancedInputActionI_Pause
  (params (ActionValue :type Boolean) (ElapsedSeconds :type Float%20%28double-precision%29) (TriggeredSeconds :type Float%20%28double-precision%29) (InputAction :type Input%20Action%20Object%20Reference :default "/Game/Marco/Player/Input/I_Pause.I_Pause"))
  (:Started
    (if (Game|IsGamePaused)
      (Utilities|IsValid (Variables|Default|GetWG_pause)
        (:Is%20Valid
          (Widget|RemovefromParent (Variables|Default|GetWG_pause))
          (Variables|Default|SetbShowMouseCursor false)
          (Game|SetGamePaused false)
          (bind _asbp_gm_gameplay (Utilities|Casting|CastToBP_GM_Gameplay (Game|GetGameMode)))
          (Default|TogglePause _asbp_gm_gameplay false)))
      (else
        (Utilities|IsValid (Variables|Default|GetWG_pause)
          (:Is%20Valid
            _)
          (:Is%20Not%20Valid
            (bind _returnvalue (UserInterface|CreateWidget "/Game/Marco/HUD/BPs/WG_PauseMenu.WG_PauseMenu_C"))
            (Variables|Default|SetWG_pause _returnvalue)))
        (UserInterface|Viewport|AddtoViewport (Variables|Default|GetWG_pause) 0)
        (Variables|Default|SetbShowMouseCursor true)
        (bind _asbp_gm_gameplay_2 (Utilities|Casting|CastToBP_GM_Gameplay (Game|GetGameMode)))
        (Default|TogglePause _asbp_gm_gameplay_2 true)
        (Game|SetGamePaused true)))))

(event EventBeginPlay
  (bind _self self)
  (bind _returnvalue (PlayerController|LocalPlayerSubsystems|GetEnhancedInputLocalPlayerSubsystem _self))
  (Utilities|IsValid _returnvalue
    (:Is%20Valid
      (Input|AddMappingContext _returnvalue "/Game/Marco/Player/Input/IM_Multiplayer.IM_Multiplayer" 0 "(bIgnoreAllPressedKeysUntilRelease=True,bForceImmediately=False)")
      (CallFunction|CachePlayerPawn)
      (CallFunction|UpdateCamera))))

(fn ConstructionScript)
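; BP_Player is a player character that moves on fixed world axes, interacts with nearby BP_Interactuable actors and can be stunned.
; Move inputs turn it toward the pressed axis, while Tick toggles Niagara with velocity; UpdateRotation is effectively empty.
; A Sphere overlap drives guide messages and supplies the target for two interact actions that pass carry state.
; HitByStun, also on key X, plays a fall and briefly locks movement.
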(event OnComponentBeginOverlap(Sphere)
  (params (OverlappedComponent :type Primitive%20Component%20Object%20Reference) (OtherActor :type Actor%20Object%20Reference) (OtherComp :type Primitive%20Component%20Object%20Reference) (OtherBodyIndex :type Integer) (bFromSweep :type Boolean) (SweepResult :type Hit%20Result%20Structure%20%28by%20ref%29))
  (if (Utilities|DoesObjectImplementInterface OtherActor "/Game/Marco/Interactuables/Base/CanBeInteracted.CanBeInteracted_C")
    (Class|CanbeInteracted|ShowGuide(Message) OtherActor (Variables|Default|Getcarryable))))

(event OnComponentEndOverlap(Sphere)
  (params (OverlappedComponent :type Primitive%20Component%20Object%20Reference) (OtherActor :type Actor%20Object%20Reference) (OtherComp :type Primitive%20Component%20Object%20Reference) (OtherBodyIndex :type Integer))
  (if (Utilities|DoesObjectImplementInterface OtherActor "/Game/Marco/Interactuables/Base/CanBeInteracted.CanBeInteracted_C")
    (Class|CanbeInteracted|HideGuide(Message) OtherActor)))

(event Custom|MoveRight
  (params (scale :type Float%20%28double-precision%29))
  (if (Variables|Default|GetcanMove)
    (Pawn|Input|AddMovementInput "0.000000,1.000000,0.000000" scale false)
    (if (not (== scale 0.0))
      (Transformation|SetActorRelativeRotation (Math|Interpolation|RInterpTo (Transformation|GetActorRotation) (Math|Conversions|RotationFromXVector (* (Math|Float|Sign(Float) scale) "0.000000,1.000000,0.000000")) (Utilities|Time|GetWorldDeltaSeconds) (Variables|Default|GetInterp%20Speed))))))

(event Custom|MoveUp
  (params (scale :type Float%20%28double-precision%29))
  (if (Variables|Default|GetcanMove)
    (Pawn|Input|AddMovementInput "1.000000,0.000000,0.000000" scale false)
    (if (not (== scale 0.0))
      (Transformation|SetActorRelativeRotation (Math|Interpolation|RInterpTo (Transformation|GetActorRotation) (Math|Conversions|RotationFromXVector (* "1.000000,0.000000,0.000000" (Math|Float|Sign(Float) scale))) (Utilities|Time|GetWorldDeltaSeconds) (Variables|Default|GetInterp%20Speed))))))

(event Custom|ActionA
  (bind _array_element (Utilities|Array|ForEachLoopwithBreak (Collision|GetOverlappingActors (Variables|Default|GetSphere) "/Game/Marco/Interactuables/Base/BP_Interactuable.BP_Interactuable_C" :!class /Script/Engine.PrimitiveComponent) :!label _label)
    (:LoopBody
      (Class|CanbeInteracted|Interact(Message) _array_element (Variables|Default|GetisCarrying) self true)
      (goto _label Break))))

(event Custom|ActionB
  (bind _array_element (Utilities|Array|ForEachLoopwithBreak (Collision|GetOverlappingActors (Variables|Default|GetSphere) "/Game/Marco/Interactuables/Base/BP_Interactuable.BP_Interactuable_C" :!class /Script/Engine.PrimitiveComponent) :!label _label)
    (:LoopBody
      (Class|CanbeInteracted|Interact(Message) _array_element (Variables|Default|GetisCarrying) self false)
      (goto _label Break))))

(event Custom|DisableMovement
  (Components|Movement|StopMovementImmediately (Variables|Character|GetCharacterMovement))
  (Variables|Default|SetcanMove false))

(event Custom|EnableMovement
  (Variables|Default|SetcanMove true))

(event Custom|HitByStun
  ;[1 1 1] Play falling anim
  (bind _returnvalue (Animation|PlayAnimMontage "/Game/Otros/Caida_fix_Anim_Montage.Caida_fix_Anim_Montage" 1.0 "None"))
  (Audio|PlaySound2D "/Game/Audio/MS_Caida.MS_Caida" 1.0 1.0 0.0 0 0)
  (Utilities|FlowControl|Delay (/ _returnvalue 3.0))
  (CallFunction|DisableMovement)
  (Utilities|FlowControl|Delay (* (/ _returnvalue 3.0) 2.0))
  (CallFunction|EnableMovement))

(event Custom|ToggleArrow
  (params (activate :type Boolean))
  (bind _as_wg_arrow_down (Variables|Default|GetAs%20WG%20Arrow%20Down))
  (if activate
    (Default|DoAnimation _as_wg_arrow_down)
    (else
      (Default|StopA _as_wg_arrow_down))))

(event EventTick
  (params (DeltaSeconds :type Float%20%28single-precision%29))
  (bind _niagara (Variables|Default|GetNiagara))
  (Utilities|FlowControl|Sequence
    (:then_0
      (CallFunction|UpdateRotation DeltaSeconds))
    (:then_1
      (if (Utilities|Operators|EqualEqual :A (Transformation|GetVelocity))
        (Components|Activation|Deactivate _niagara)
        (else
          (Components|Activation|Activate _niagara false))))))

(event EventBeginPlay
  (bind _aswg_arrow_down (Utilities|Casting|CastToWG_ArrowDown (UserInterface|GetWidget (Variables|Default|GetWidget))))
  (Variables|Default|SetAs%20WG%20Arrow%20Down _aswg_arrow_down))

(event Input|KeyboardEvents|X
  (params (Key :type Key%20Structure :default "None"))
  (:Pressed
    (CallFunction|HitbyStun)))

(fn ConstructionScript)

(fn UpdateRotation
  (params (DeltaTime :type Float%20%28single-precision%29)))